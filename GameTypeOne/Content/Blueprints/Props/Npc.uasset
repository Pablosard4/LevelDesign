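; NPC guard that either patrols a loop of four target points or holds its start position, and chases the player on sight.
; PawnSensing starts an AI move toward the player and immediately calls Chased, which prints a caught message.
; Tick re-issues patrol or return moves while Patroling is set, and clears Saw once player distance exceeds sight radius.
; Sighting clears Patroling, which is never restored afterward.
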(event OnSeePawn(PawnSensing)
  (params (Pawn :type Pawn%20Object%20Reference))
  ;[1 0 0.09154] Seek
  (bind _asthird_person_character (Utilities|Casting|CastToThirdPersonCharacter Pawn))
  (Variables|Default|SetSaw true)
  (Variables|Default|SetPatroling false)
  (AI|AIMoveTo self "0, 0, 0" _asthird_person_character 5.0 false
    (:then
      (CallFunction|Chased))))

(event Custom|Patrol
  ;[1 0 0.07132] Patrol
  (if (Variables|Default|GetNPCPatrol)
    (AI|AIMoveTo self "0, 0, 0" (Variables|Default|GetTargetPoint1) 5.0 false
      (:OnSuccess
        (Utilities|FlowControl|Delay 0.2)
        (AI|AIMoveTo self "0, 0, 0" (Variables|Default|GetTargetPoint2) 5.0 false
          (:OnSuccess
            (Utilities|FlowControl|Delay 0.2)
            (AI|AIMoveTo self "0, 0, 0" (Variables|Default|GetTargetPoint3) 5.0 false
              (:OnSuccess
                (Utilities|FlowControl|Delay 0.2)
                (AI|AIMoveTo self "0, 0, 0" (Variables|Default|GetTargetPoint4) 5.0 false
                  (:OnSuccess
                    (CallFunction|Patrol)))))))))))

(event EventTick
  (params (DeltaSeconds :type Float%20%28single-precision%29))
  (bind _postion (Variables|Default|GetPostion))
  ;[1 0 0.06124] Check If Player Is Visible, If Not, Patrol
  (if (Variables|Default|GetSaw)
    (Utilities|FlowControl|Delay 0.2)
    (bind _visible (CallFunction|Playerisvisable))
    (if _visible
      (Variables|Default|SetSaw false)
      (else
        (Variables|Default|SetSaw true)))
    (elif (Variables|Default|GetPatroling)
      (if (Variables|Default|GetNPCPatrol)
        (Utilities|FlowControl|Delay 0.2)
        (CallFunction|Patrol)
        (Variables|Default|SetPatroling true)
        (else
          (Utilities|FlowControl|Delay 0.2)
          (Development|PrintString (Utilities|String|ToString(Vector) _postion))
          (AI|AIMoveTo self _postion 0 5.0 false))))))

(event EventBeginPlay
  (bind _charactermovement (Variables|Character|GetCharacterMovement))
  ;[1 0 0.1577] Start Logic
  (CallFunction|Patrol)
  (Variables|Default|SetPostion (Transformation|GetActorLocation self))
  (Variables|Default|SetPatroling true)
  (Variables|/Script/Engine.CharacterMovementComponent|SetMaxWalkSpeed _charactermovement (* (Variables|Default|GetSpeed) (Class|MovementComponent|GetMaxSpeed _charactermovement))))

(fn ConstructionScript)

(fn Playerisvisable
  (return (> (Transformation|GetDistanceTo (Game|Player|GetPlayerPawn 0)) (Variables|/Script/AIModule.PawnSensingComponent|GetSightRadius (Variables|Default|GetPawnSensing)))))

(fn Chased
  (Utilities|Casting|CastToThirdPersonCharacter (Game|GetPlayerCharacter 0))
  (Development|PrintString "Te pillaron")
  (return))